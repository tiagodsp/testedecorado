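; Game mode for a furniture decorating test that loads the furniture catalogue and shows the main interface.
; On BeginPlay it reads every row of the FurnitureData table into a Furnitures array.
; It then creates the HUD widget, casts it to W_MainInterface, passes it the furniture list and adds it to the viewport.
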(event EventBeginPlay
  (Utilities|FlowControl|Sequence
    (:then_0
      ;[0 1 0.09554] Get furniture data from database
      (bind _outrownames (DataTable|GetDataTableRowNames "/Game/Blueprints/FurnitureData.FurnitureData"))
      (for _array_element _outrownames
        (bind _returnvalue (Utilities|GetDataTableRow "/Game/Blueprints/FurnitureData.FurnitureData" _array_element)
          (:then
            (Utilities|Array|Add (Variables|Default|GetFurnitures) _returnvalue)))))
    (:then_1
      ;[0 0.1229 1] Display UI
      (bind _returnvalue_2 (UserInterface|CreateWidget (Variables|Default|GetHUD)))
      (bind _asw_main_interface (Utilities|Casting|CastToW_MainInterface _returnvalue_2))
      (bind _output_get (Variables|Default|SetUIWidget _asw_main_interface))
      (Default|SetObjectList _output_get (Variables|Default|GetFurnitures))
      (UserInterface|Viewport|AddtoViewport _output_get 0))))

(fn ConstructionScript)