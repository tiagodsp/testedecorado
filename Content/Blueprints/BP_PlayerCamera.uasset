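; Player camera pawn for furniture decorating, with axis movement and spawning from number keys or UI item selection.
; Tick projects the mouse onto surfaces as a 3D cursor, frozen while the options menu is open.
; An enum state machine (Idle, WaitingOption, Transform, Release) routes clicks between selecting furniture, pressing the world-space menu and confirming transforms.
; Menu options move or rotate furniture toward the cursor, delete, cycle textures or call WebSocket rotation sync.
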(event Custom|SpawnObjectAtCursor
  (params (ObjectItem :type S%20Object%20Item%20Structure))
  ;[1 0.9581 0] Spawn object at cursor position
  (bind _returnvalue (Game|SpawnActorfromClass "/Game/Blueprints/FurnitureObject.FurnitureObject_C" (Math|Transform|MakeTransform (Transformation|GetWorldLocation (Variables|Default|GetCursorRoot)) "0, 0, 0" "1,1,1") "Undefined" 0 ObjectItem 0))
  (Variables|Default|SetSelectedObject _returnvalue))

(event Custom|OnObjectMenuSelectedOption
  (params (Move :type Boolean) (Rotate :type Boolean) (Delete :type Boolean) (NextTexture :type Boolean) (PreviousTexture :type Boolean) (Sync :type Boolean) (Close :type Boolean))
  ;[1 0.4745 0.07292] Check selected menu option
  (bind _output_get (Variables|Default|SetIsTranformModeMoveOn Move))
  (bind _output_get_2 (Variables|Default|SetIsTransformModeRotateOn Rotate))
  (if Delete
    (Actor|DestroyActor (Variables|Default|GetSelectedObject))
    (Variables|Default|SetSelectedObject 0)
    (Variables|StateControl|SetIsObjectDeleted true)
    (elif NextTexture
      (CallFunction|NextTexture)
      (elif PreviousTexture
        (CallFunction|PreviousTexture)
        (elif Close
          (Variables|StateControl|SetIsMenuClosed true)
          (elif Sync
            (Default|EnableSyncRotationwithWebSocket (Variables|Default|GetSelectedObject) false)
            (else
              (Variables|StateControl|SetIsTransformModeEnabled (or _output_get_2 _output_get)))))))))

(event Custom|NewObjectCreated
  (params (ObjectItem :type S%20Object%20Item%20Structure))
  (CallFunction|SpawnObjectatCursor ObjectItem)
  (Variables|StateControl|SetIsNewObjectCreated true)
  (Variables|StateControl|SetIsTransformModeEnabled true)
  (Variables|Default|SetIsTranformModeMoveOn true))

(event Custom|NextTexture
  (bind _selectedobject (Variables|Default|GetSelectedObject))
  ;[0.8595 0 1] Set textures at the current object
  (Utilities|IsValid _selectedobject
    (:Is%20Valid
      (Default|NextTexture _selectedobject))))

(event Custom|PreviousTexture
  (bind _selectedobject (Variables|Default|GetSelectedObject))
  ;[0.8595 0 1] Set textures at the current object
  (Utilities|IsValid _selectedobject
    (:Is%20Valid
      (Default|PreviousTexture _selectedobject))))

(event EventTick
  (params (DeltaSeconds :type Float%20%28single-precision%29))
  (bind _returnvalue (Game|GetPlayerController 0))
  (bind _cursorroot (Variables|Default|GetCursorRoot))
  (bind _selectedobject (Variables|Default|GetSelectedObject))
  (bind _selectedobject_2 (Variables|Default|GetSelectedObject))
  (bind _cursorroot_2 (Variables|Default|GetCursorRoot))
  (bind _widgetinteraction (Variables|Default|GetWidgetInteraction))
  (bind (_worldlocation _worlddirection) (Game|Player|ConvertMouseLocationToWorldSpace _returnvalue))
  (bind _returnvalue_2 (Transformation|GetWorldLocation _cursorroot_2))
  (bind _returnvalue_3 (Transformation|GetWorldLocation _cursorroot))
  (bind _rootcomponent (Variables|/Script/Engine.Actor|GetRootComponent _selectedobject_2))
  (bind _rootcomponent_2 (Variables|/Script/Engine.Actor|GetRootComponent _selectedobject))
  (bind _returnvalue_4 (Transformation|GetWorldLocation _rootcomponent_2))
  (Utilities|FlowControl|Sequence
    (:then_0
      ;[0 1 0.9612] Get UI Widget
      (bind _asteste_decorado_game_mode (Utilities|Casting|CastToTesteDecoradoGameMode (Game|GetGameMode)))
      (bind _output_get (Variables|Default|SetUIWidget (Variables|/Game/Blueprints/TesteDecoradoGameMode.TesteDecoradoGameMode_C|GetUIWidget _asteste_decorado_game_mode)))
      (EventDispatchers|BindEventtoObjectSelected _output_get (EventDispatchers|CreateEvent :!event Custom|NewObjectCreated)))
    (:then_1
      ;[0.1101 0.2339 1] Set 3D cursor position
      (if (Variables|Default|GetIsObjectMenuOpened)
        ;;[1 1 1] Fixes cursor at the same position when camera moves
        (Transformation|SetWorldLocation (Variables|Default|GetCursorRoot) (Variables|Default|GetLastCursorLocation) false false)
        (else
          (bind (_outhit _returnvalue_5) (Collision|LineTraceByChannel _worldlocation (+ _worldlocation (* _worlddirection 1e+04)) "TraceTypeQuery1" false 0 "None"))
          (if _returnvalue_5
            (Transformation|SetWorldLocation (Variables|Default|GetCursorRoot) (.location _outhit) false false)
            (Transformation|SetWorldRotation (Variables|Default|GetCursorRoot) (Math|Rotator|FindLookatRotation (.location _outhit) (+ (.location _outhit) (* (.normal _outhit) 1e+03))) false false)
            ;;[1 1 1] Stores last cursor position
            (Variables|Default|SetLastCursorLocation (.location _outhit))
            (else
              (Transformation|SetWorldLocation (Variables|Default|GetCursorRoot) (Variables|Default|GetLastCursorLocation) false false)
              (Transformation|SetWorldRotation (Variables|Default|GetCursorRoot) "0, 0, 0" false false))))))
    (:then_2
      (if (Variables|StateControl|GetIsTransformModeEnabled)
        (Utilities|IsValid (Variables|Default|GetSelectedObject)
          (:Is%20Valid
            (Utilities|FlowControl|Sequence
              (:then_0
                ;[0.9427 0.3103 1] Move object
                (if (Variables|Default|GetIsTranformModeMoveOn)
                  (Transformation|SetWorldLocation _rootcomponent (Math|Vector|MakeVector (.x _returnvalue_2) (.y _returnvalue_2) (.z (Transformation|GetWorldLocation _rootcomponent))) false false)))
              (:then_1
                ;[0 1 0.5069] Rotate Object
                (if (Variables|Default|GetIsTransformModeRotateOn)
                  (Transformation|SetWorldRotation _rootcomponent_2 (Math|Rotator|FindLookatRotation (Math|Vector|MakeVector (.x _returnvalue_4) (.y _returnvalue_4) (.z _returnvalue_4)) (Math|Vector|MakeVector (.x _returnvalue_3) (.y _returnvalue_3) (.z _returnvalue_4))) false false))))))))
    (:then_3
      ;[0.9566 1 0.08689] Update widget interaction cursor direction
      (Transformation|SetWorldRotation (Variables|Default|GetOptionsMenuWidget) (Math|Rotator|FindLookatRotation (Transformation|GetWorldLocation (Variables|Default|GetOptionsMenuWidget)) (Transformation|GetWorldLocation (Variables|Transformation|GetRootComponent))) false false)
      (Transformation|SetWorldRotation _widgetinteraction (Math|Rotator|FindLookatRotation (Transformation|GetWorldLocation _widgetinteraction) (.WorldLocation (Game|Player|ConvertMouseLocationToWorldSpace (Game|GetPlayerController 0)))) false false))
    (:then_4
      ;[1 0 0.05075] Update state transistions
      (switch Utilities|FlowControl|Switch|SwitchonObjectSelectionStates (Variables|StateControl|GetObjectSelectionState)
        (:NewEnumerator0
          (if (Variables|StateControl|GetIsObjectSelected)
            (Variables|StateControl|SetObjectSelectionState "NewEnumerator1")
            (elif (Variables|StateControl|GetIsNewObjectCreated)
              (Variables|StateControl|SetObjectSelectionState "NewEnumerator2")
              (else
                (Variables|StateControl|SetObjectSelectionState "NewEnumerator0")))))
        (:NewEnumerator1
          (if (Variables|StateControl|GetIsTransformModeEnabled)
            (Variables|StateControl|SetObjectSelectionState "NewEnumerator2")
            (CallFunction|SetDisplayObjectMenu false)
            (elif (or (Variables|StateControl|GetIsObjectDeleted) (Variables|StateControl|GetIsMenuClosed))
              (Variables|StateControl|SetObjectSelectionState "NewEnumerator4"))))
        (:NewEnumerator2
          (if (Variables|Default|GetIsObjectTransformed)
            (Variables|StateControl|SetObjectSelectionState "NewEnumerator4")))
        (:NewEnumerator4
          (Variables|StateControl|SetObjectSelectionState "NewEnumerator0")
          (Variables|Default|SetIsObjectTransformed false)
          (Variables|StateControl|SetIsTransformModeEnabled false)
          (Variables|StateControl|SetIsObjectSelected false)
          (Variables|StateControl|SetIsObjectDeleted false)
          (Variables|StateControl|SetIsMenuClosed false)
          (Variables|StateControl|SetIsNewObjectCreated false)
          (CallFunction|SetDisplayObjectMenu false))))))

(event EventBeginPlay
  ;[0.5728 1 0.9901] Bind event of the Object Options Menu
  (bind _asw_object_options_menu (Utilities|Casting|CastToW_ObjectOptionsMenu (UserInterface|GetUserWidgetObject (Variables|Default|GetOptionsMenuWidget))))
  (EventDispatchers|BindEventtoSelectedOption _asw_object_options_menu (EventDispatchers|CreateEvent :!event Custom|OnObjectMenuSelectedOption))
  (CallFunction|SetDisplayObjectMenu false))

(event Input|AxisEvents|InputAxisMoveFoward
  (params (AxisValue :type Float%20%28single-precision%29))
  (bind _fowardarrow (Variables|Default|GetFowardArrow))
  (bind _returnvalue (Math|Vector|GetForwardVector _fowardarrow))
  (bind _returnvalue_2 (* _returnvalue 1e+02))
  ;[0 0.9157 1] Movement
  (Pawn|Input|AddMovementInput (Math|Vector|MakeVector (.x _returnvalue_2) (.y _returnvalue_2) 0.0) AxisValue false))

(event Input|AxisEvents|InputAxisMoveRight
  (params (AxisValue :type Float%20%28single-precision%29))
  (bind _fowardarrow (Variables|Default|GetFowardArrow))
  (bind _returnvalue (Math|Vector|GetForwardVector _fowardarrow))
  (bind _returnvalue_2 (* _returnvalue 1e+02))
  ;[0 0.9157 1] Movement
  (Pawn|Input|AddMovementInput (Math|Vector|MakeVector (.y _returnvalue_2) (.x _returnvalue_2) 0.0) AxisValue false))

(event Input|KeyboardEvents|1
  (params (Key :type Key%20Structure))
  (bind _uiwidget (Variables|Default|GetUIWidget))
  ;[0.5685 0 1] Keyboard Shortcuts
  (:Pressed
    (Default|SetActiveItemIndex _uiwidget)
    (bind _objectitem (Default|GetObjectbyIndex _uiwidget))
    (CallFunction|SpawnObjectatCursor _objectitem)))

(event Input|KeyboardEvents|4
  (params (Key :type Key%20Structure))
  (bind _uiwidget (Variables|Default|GetUIWidget))
  ;[0.5685 0 1] Keyboard Shortcuts
  (:Pressed
    (Default|SetActiveItemIndex _uiwidget 3)
    (bind _objectitem (Default|GetObjectbyIndex _uiwidget 3))
    (CallFunction|SpawnObjectatCursor _objectitem)))

(event Input|KeyboardEvents|Up
  (params (Key :type Key%20Structure))
  (bind _selectedobject (Variables|Default|GetSelectedObject))
  ;[0.8595 0 1] Set textures at the current object
  (:Pressed
    (Utilities|IsValid _selectedobject
      (:Is%20Valid
        (Default|NextTexture _selectedobject)))))

(event Input|KeyboardEvents|Down
  (params (Key :type Key%20Structure))
  (bind _selectedobject (Variables|Default|GetSelectedObject))
  ;[0.8595 0 1] Set textures at the current object
  (:Pressed
    (Utilities|IsValid _selectedobject
      (:Is%20Valid
        (Default|PreviousTexture _selectedobject)))))

(event Input|MouseEvents|LeftMouseButton
  (params (Key :type Key%20Structure))
  (bind _cursorroot (Variables|Default|GetCursorRoot))
  (bind _widgetinteraction (Variables|Default|GetWidgetInteraction))
  (bind _returnvalue (Transformation|GetWorldLocation _cursorroot))
  ;[0 0.9758 1] Click functions based on current state
  (:Pressed
    (switch Utilities|FlowControl|Switch|SwitchonObjectSelectionStates (Variables|StateControl|GetObjectSelectionState)
      (:NewEnumerator0
        (bind _outhit (Collision|SphereTraceByChannel _returnvalue _returnvalue 5.0 "TraceTypeQuery1" false 0 "None"))
        (bind _asfurniture_object (Utilities|Casting|CastToFurnitureObject (.hitactor _outhit))
          (:then
            (Variables|Default|SetSelectedObject _asfurniture_object)
            (Variables|StateControl|SetIsObjectSelected true)
            (CallFunction|SetDisplayObjectMenu true))
          (:CastFailed
            (Variables|Default|SetSelectedObject 0)
            (Variables|StateControl|SetIsObjectSelected false)
            (CallFunction|SetDisplayObjectMenu false))))
      (:NewEnumerator1
        (Class|WidgetInteractionComponent|PressPointerKey _widgetinteraction "LeftMouseButton")
        (Class|WidgetInteractionComponent|ReleasePointerKey _widgetinteraction "LeftMouseButton"))
      (:NewEnumerator2
        (Variables|Default|SetIsObjectTransformed true)))))

(event Input|KeyboardEvents|5
  (params (Key :type Key%20Structure))
  (bind _uiwidget (Variables|Default|GetUIWidget))
  ;[0.5685 0 1] Keyboard Shortcuts
  (:Pressed
    (Default|SetActiveItemIndex _uiwidget 4)
    (bind _objectitem (Default|GetObjectbyIndex _uiwidget 4))
    (CallFunction|SpawnObjectatCursor _objectitem)))

(event Input|KeyboardEvents|2
  (params (Key :type Key%20Structure))
  (bind _uiwidget (Variables|Default|GetUIWidget))
  ;[0.5685 0 1] Keyboard Shortcuts
  (:Pressed
    (Default|SetActiveItemIndex _uiwidget 1)
    (bind _objectitem (Default|GetObjectbyIndex _uiwidget 1))
    (CallFunction|SpawnObjectatCursor _objectitem)))

(event Input|KeyboardEvents|3
  (params (Key :type Key%20Structure))
  (bind _uiwidget (Variables|Default|GetUIWidget))
  ;[0.5685 0 1] Keyboard Shortcuts
  (:Pressed
    (Default|SetActiveItemIndex _uiwidget 2)
    (bind _objectitem (Default|GetObjectbyIndex _uiwidget 2))
    (CallFunction|SpawnObjectatCursor _objectitem)))

(event Input|KeyboardEvents|6
  (params (Key :type Key%20Structure))
  (bind _uiwidget (Variables|Default|GetUIWidget))
  ;[0.5685 0 1] Keyboard Shortcuts
  (:Pressed
    (Default|SetActiveItemIndex _uiwidget 5)
    (bind _objectitem (Default|GetObjectbyIndex _uiwidget 5))
    (CallFunction|SpawnObjectatCursor _objectitem)))

(event Input|KeyboardEvents|7
  (params (Key :type Key%20Structure))
  (bind _uiwidget (Variables|Default|GetUIWidget))
  ;[0.5685 0 1] Keyboard Shortcuts
  (:Pressed
    (Default|SetActiveItemIndex _uiwidget 6)
    (bind _objectitem (Default|GetObjectbyIndex _uiwidget 6))
    (CallFunction|SpawnObjectatCursor _objectitem)))

(event Input|KeyboardEvents|8
  (params (Key :type Key%20Structure))
  (bind _uiwidget (Variables|Default|GetUIWidget))
  ;[0.5685 0 1] Keyboard Shortcuts
  (:Pressed
    (Default|SetActiveItemIndex _uiwidget 7)
    (bind _objectitem (Default|GetObjectbyIndex _uiwidget 7))
    (CallFunction|SpawnObjectatCursor _objectitem)))

(event Input|KeyboardEvents|9
  (params (Key :type Key%20Structure))
  (bind _uiwidget (Variables|Default|GetUIWidget))
  ;[0.5685 0 1] Keyboard Shortcuts
  (:Pressed
    (Default|SetActiveItemIndex _uiwidget 8)
    (bind _objectitem (Default|GetObjectbyIndex _uiwidget 8))
    (CallFunction|SpawnObjectatCursor _objectitem)))

(fn ConstructionScript)

(fn SetDisplayObjectMenu
  (params (DisplayMenu :type Boolean))
  (bind _optionsmenuwidget (Variables|Default|GetOptionsMenuWidget))
  (bind _output_get (Variables|Default|SetIsObjectMenuOpened DisplayMenu))
  (if _output_get
    (Rendering|SetVisibility _optionsmenuwidget true false)
    (else
      (Rendering|SetVisibility _optionsmenuwidget false false))))