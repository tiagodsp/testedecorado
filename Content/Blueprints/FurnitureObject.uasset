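; Furniture actor whose construction script applies mesh and initial transform from FurnitureData.
; An optional WebSocket, updated each tick while connected, sets the actor root's yaw from incoming messages.
; EnableSyncRotationWithWebSocket toggles the connection through a FlipFlop, ignoring its Enable argument.
; Next/PreviousTexture step through FurnitureData materials on a configured slot, while SetHighlight is an empty TODO.
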(event OnMessage(WebSocket)
  (params (Data :type String))
  ;[0 0.139 1] Rotate object with information from WebSocket server
  (Transformation|SetWorldRotation (Variables|Default|GetDefaultSceneRoot) (Math|Rotator|MakeRotator 0.0 0.0 (Math|Conversions|ToFloat(Integer) Data)) false false))

(event Custom|SetHighlight
  (params (Highlight :type Boolean))
  ;[1 0 0.02787] TODO - Create highlight effect
)

(event Custom|EnableSyncRotationWithWebSocket
  (params (Enable :type Boolean))
  (bind _websocket (Variables|Default|GetWebSocket))
  ;[1 0 0.05887] Enable/Disable connection with WebSocket
  (bind _isa (Utilities|FlowControl|FlipFlop)
    (:A
      _)
    (:B
      _))
  (bind _output_get (Variables|Default|SetIsWebSocketConnected _isa))
  (if _output_get
    (Class|WebSocketComponent|DefaultConnect _websocket)
    (else
      (Class|WebSocketComponent|Disconnect _websocket))))

(event Custom|NextTexture
  (bind _furnituredata (Variables|Configuration|GetFurnitureData))
  ;[1 0.8839 0] Set next texture
  (if (< (Variables|Default|GetCurrentTextureIndex) (Utilities|Array|Length (.materials _furnituredata)))
    (Rendering|Material|SetMaterial (Variables|Default|GetStaticMesh) (.changematerialindex _furnituredata) (Utilities|Array|Get(acopy) (.materials _furnituredata) (Variables|Default|GetCurrentTextureIndex)))
    (bind _output_get (Variables|Default|SetCurrentTextureIndex (+ (stale _output_get) 1)))))

(event Custom|PreviousTexture
  (bind _furnituredata (Variables|Configuration|GetFurnitureData))
  ;[0.0926 1 0] Set previous texture
  (if (>= (Variables|Default|GetCurrentTextureIndex) 0)
    (Rendering|Material|SetMaterial (Variables|Default|GetStaticMesh) (.changematerialindex _furnituredata) (Utilities|Array|Get(acopy) (.materials _furnituredata) (Variables|Default|GetCurrentTextureIndex)))
    (bind _output_get (Variables|Default|SetCurrentTextureIndex (+ (stale _output_get) -1)))))

(event EventBeginPlay
  ;[1 0.7887 0] Check if sync with webscoket at begin play
  (if (Variables|Default|GetEnableWebSocket)
    (CallFunction|EnableSyncRotationwithWebSocket false)))

(event EventTick
  (params (DeltaSeconds :type Float%20%28single-precision%29))
  ;[1 0 0.7545] Update WebSocket data
  (if (Variables|Default|GetIsWebSocketConnected)
    (Class|WebSocketComponent|Update (Variables|Default|GetWebSocket))))

(fn ConstructionScript
  (bind _furnituredata (Variables|Configuration|GetFurnitureData))
  (Components|StaticMesh|SetStaticMesh (Variables|Default|GetStaticMesh) (.mesh _furnituredata))
  (Transformation|SetRelativeTransform (Variables|Default|GetObjectMeshRoot) (.initialtransform _furnituredata) false false))